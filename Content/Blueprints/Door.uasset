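; Interactable door actor that swings open and shut around its yaw axis.
; At BeginPlay it binds DoorAnimation to the interact delegate of its PInteractable.
; Each interaction toggles IsClosed and plays or reverses the DoorAnim timeline, whose track scales the static mesh's relative yaw up to a quarter turn.
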(event `self.ReceiveBeginPlay`
  (add `PInteractableComponent.OnInteractDelegate` (`self.PInteractable`) (delegate `DoorAnimation`)))

(event `DoorAnimation`
  (params (Cause :type "PCharacter Object Reference"))
  (if (`self.IsClosed`)
    (set `self.IsClosed` false)
    (bind (_direction _newtrack_0) (`Timeline|DoorAnim` :!label _label)
      (:`Update`
        (`SceneComponent.K2_SetRelativeRotation` (`self.StaticMesh`) (`KismetMathLibrary.MakeRotator` 0.0 0.0 (* _newtrack_0 90.0)) false false)))
    (else
      (set `self.IsClosed` true)
      (goto _label :!via `Reverse`))))

(fn `UserConstructionScript`)