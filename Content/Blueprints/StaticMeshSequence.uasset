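; StaticMeshSequence is an actor that lays out a row of copies of one static mesh along local X, up to its End component.
; The construction script sizes the mesh from its bounding box, then adds Instanced Static Mesh instances spaced by that width plus a non-negative gap.
; Each instance transform takes location, rotation and scale offsets from GenerateRandomValues, fed by min/max ranges and a RandomStream.
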(event `self.ReceiveBeginPlay`)

(fn `CanSpawnMeshInstance`
  (returns (CanSpawn :type Boolean))
  (return (> (.x (`SceneComponent.RelativeLocation` (`self.End`))) (* (`InstancedStaticMeshComponent.GetInstanceCount` (`self.InstancedStaticMesh`)) (+ (`self.MeshSize`) (`self.MeshOffset`))))))

(fn `GenerateRandomOffset`
  (returns (Location :type "Vector Structure") (Rotation :type "Rotator Structure") (Scale :type "Vector Structure"))
  (bind (_x _y _z) (`self.GenerateRandomValues` (.x (`self.LocationOffsetMin`)) (.x (`self.LocationOffsetMax`)) (.y (`self.LocationOffsetMin`)) (.y (`self.LocationOffsetMax`)) (.z (`self.LocationOffsetMin`)) (.z (`self.LocationOffsetMax`)) (`self.RandomStream`)))
  (bind (_x_2 _y_2 _z_2) (`self.GenerateRandomValues` (.x (`self.ScaleOffsetMin`)) (.x (`self.ScaleOffsetMax`)) (.y (`self.ScaleOffsetMin`)) (.y (`self.ScaleOffsetMax`)) (.z (`self.ScaleOffsetMin`)) (.z (`self.ScaleOffsetMax`)) (`self.RandomStream`)))
  (bind (_x_3 _y_3 _z_3) (`self.GenerateRandomValues` (.roll (`self.RotationOffsetMin`)) (.roll (`self.RotationOffsetMax`)) (.pitch (`self.RotationOffsetMin`)) (.pitch (`self.RotationOffsetMax`)) (.yaw (`self.RotationOffsetMin`)) (.yaw (`self.RotationOffsetMax`)) (`self.RandomStream`)))
  (return (`KismetMathLibrary.MakeVector` _x _y _z) (`KismetMathLibrary.MakeRotator` _x_3 _y_3 _z_3) (`KismetMathLibrary.MakeVector` _x_2 _y_2 _z_2)))

(fn `Init`
  (`|ExecutionSequence`
    (:`then_0`
      (`self.InitVariables`))
    (:`then_1`
      (`/Engine/EditorBlueprintResources/StandardMacros.IsValid` (`self.Mesh`)
        (:`Is Valid`
          (while (`self.CanSpawnMeshInstance`)
            (`self.SpawnMeshInstance`)))))))

(fn `InitVariables`
  (bind _meshoffset (`self.MeshOffset`))
  (bind (_min _max) (break `Box` (`StaticMesh.GetBoundingBox` (`self.Mesh`))))
  (`|ExecutionSequence`
    (:`then_0`
      ;[1 1 1] Set Mesh Size
      (set `self.MeshSize` (.x (- _max _min))))
    (:`then_1`
      ;[1 1 1] Set Mesh Offset
      (set `self.MeshOffset` (`KismetMathLibrary.FClamp` _meshoffset 0.0 _meshoffset)))
    (:`then_2`
      ;[1 1 1] Set Instanced Static Mesh
      (`StaticMeshComponent.SetStaticMesh` (`self.InstancedStaticMesh`) (`self.Mesh`)))))

(fn `SpawnMeshInstance`
  (bind (_location _rotation _scale) (`self.GenerateRandomOffset`))
  (`InstancedStaticMeshComponent.AddInstance` (`self.InstancedStaticMesh`) (`KismetMathLibrary.MakeTransform` (+ (`KismetMathLibrary.MakeVector` (* (`InstancedStaticMeshComponent.GetInstanceCount` (`self.InstancedStaticMesh`)) (+ (`self.MeshOffset`) (`self.MeshSize`)))) _location) _rotation _scale)))

(fn `UserConstructionScript`
  (`self.Init`))